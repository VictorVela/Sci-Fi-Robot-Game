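; Interactable openable furniture prop whose construction script configures it as a locker or wardrobe by FurnitureType, setting meshes, AnimBP, trigger and anchor points.
; Trigger overlap shows a prompt widget to an eligible player, retrying on a timer if refused; a looping timer pins it to WidgetOrigin on screen.
; Interaction interface functions supply config and type-specific gameplay tags, and track the open-montage state that removes and blocks the prompt.
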(event `self.Trigger.OnComponentBeginOverlap`
  (params (OverlappedComponent :type "PrimitiveComponent Object Reference") (OtherActor :type "Actor Object Reference") (OtherComp :type "PrimitiveComponent Object Reference") (OtherBodyIndex :type Integer) (bFromSweep :type Boolean) (SweepResult :type "HitResult Structure (by ref)"))
  ;[1 1 1] Interaction Widget
  (`self.Widget-Generate` OtherActor))

(event `self.Trigger.OnComponentEndOverlap`
  (params (OverlappedComponent :type "PrimitiveComponent Object Reference") (OtherActor :type "Actor Object Reference") (OtherComp :type "PrimitiveComponent Object Reference") (OtherBodyIndex :type Integer))
  ;[1 1 1] Interaction Widget
  (`self.Widget-Destroy` :!label _label))

(event `self.ReceiveDestroyed`
  ;[1 1 1] Interaction Widget
  (goto _label))

(event `Widget Update Event`
  ;[1 1 1] Interaction Widget
  (`self.Widget-Update`))

(event `CheckWhdgetWhenInTrigger`
  (bind _overlappingactors (`PrimitiveComponent.GetOverlappingActors` (`self.Trigger`) "/Script/Engine.Character"))
  ;[1 1 1] Interaction Widget
  (if (> (`KismetArrayLibrary.Array_Length` _overlappingactors) 0)
    (`self.Widget-Generate` (`|GetArrayItem` _overlappingactors))))

(event `/Game/AdvancedLocomotionV4/Blueprints/Interfaces/Interactive_Objects_Interface.BPI_SetInteractionState`
  (params (StartedInteract :type Boolean) (Param :type Boolean))
  (set `self.StartedOpenMontage` StartedInteract)
  (`self.Widget-Destroy`))

(fn `BPI_ActorStartedInteraction`
  (returns (ReturnValue :type Boolean))
  (return (`self.StartedOpenMontage`)))

(fn `BPI_ConfigHoldingOption`
  (returns (ActorCanBeHold :type Boolean) (ActorOverlayMatch :type "/Game/AdvancedLocomotionV4/Data/Enums/ALS_OverlayState Enum"))
  (return false "NewEnumerator0"))

(fn `BPI_GetInteractionType`
  (returns (Type :type "/Game/AdvancedLocomotionV4/Data/Enums/Interaction_Type Enum"))
  (return "NewEnumerator1"))

(fn `BPI_GetInteractObjectConfig`
  (returns (CheckBasicStates :type Boolean) (UseCorrectAngle :type Boolean) (AngleArc :type "Vector2D Structure") (MaxUpPosition :type "Vector2D Structure") (MaxDistance :type "Float (double-precision)") (CheckWallHit :type Boolean) (UseOtherTrace :type Boolean) (ToIgnore :type "Array of Actor Object Reference"))
  (return true true (-65.0 65.0) (-100.0 40.0) 160.0 false false))

(fn `BPI_GetItemToPickType`
  (returns (ReturnValue :type "EIWALS_HandleItemType Enum"))
  (return "None"))

(fn `BPI_GetManualVelocity`
  (returns (Velocity :type "Vector Structure"))
  (return (0.0 0.0 0.0)))

(fn `BPI_GetObjectCollisionOverlap`
  (params (ToIgnore :type "Array of Actor Object Reference (by ref)"))
  (returns (IsOverlaping :type Boolean))
  (return false))

(fn `BPI_GetObjectTagContainer`
  (returns (ReturnValue :type "GameplayTagContainer Structure"))
  (return (select `int` (`self.FurnitureType`) :`0` (struct :`GameplayTags` (struct :`(TagName` "Interaction.OpenProp.Locker"))) :`1` (struct :`GameplayTags` (struct :`(TagName` "Interaction.OpenProp.Wardrobe"))) :!type "GameplayTagContainer Structure")))

(fn `BPI_GetObjectTraceOrigin`
  (returns (ReturnValue :type "Vector Structure"))
  (return (0.0 0.0 0.0)))

(fn `IsClosed`
  (returns (ReturnValue :type Boolean))
  (return (not (`self.StartedOpenMontage`))))

(fn `UserConstructionScript`
  (switch `int` (`self.FurnitureType`)
    (:`0`
      (`SkinnedMeshComponent.SetSkinnedAssetAndUpdate` (`self.SK_Door`) "/Game/AdvancedLocomotionV4/Props/Environment_Props/Locker/SK_Locker.SK_Locker" true)
      (`SkeletalMeshComponent.SetAnimInstanceClass` (`self.SK_Door`) "/Game/AdvancedLocomotionV4/Props/Environment_Props/Locker/SK_Locker_AnimBP.SK_Locker_AnimBP_C")
      (`SkinnedMeshComponent.SetPhysicsAsset` (`self.SK_Door`) "/Game/AdvancedLocomotionV4/Props/Environment_Props/Locker/SK_Locker_PhysicsAsset.SK_Locker_PhysicsAsset" true)
      (`BoxComponent.SetBoxExtent` (`self.Trigger`) (32.0 32.0 60.0) true)
      (`SceneComponent.K2_SetRelativeLocation` (`self.Trigger`) (0.0 -28.0 60.0) false false)
      (`StaticMeshComponent.SetStaticMesh` (`self.AdditiveMesh`) "/Game/AdvancedLocomotionV4/Props/Environment_Props/Locker/SM_Locker_Back.SM_Locker_Back")
      (`StaticMeshComponent.SetStaticMesh` (`self.AdditiveMesh2`) null)
      (`SceneComponent.K2_SetRelativeLocation` (`self.WidgetOrigin`) (16.0 -8.0 105.0) false false)
      (`SceneComponent.K2_SetRelativeLocation` (`self.TargetCharLocation`) (20.0 -54.0 0.0) false false))
    (:`1`
      (`SkinnedMeshComponent.SetSkinnedAssetAndUpdate` (`self.SK_Door`) "/Game/AdvancedLocomotionV4/Props/Environment_Props/Wardrobe/SK_Wardrobe.SK_Wardrobe" true)
      (`SkeletalMeshComponent.SetAnimInstanceClass` (`self.SK_Door`) "/Game/AdvancedLocomotionV4/Props/Environment_Props/Wardrobe/SK_Wardrobe_AnimBP.SK_Wardrobe_AnimBP_C")
      (`SkinnedMeshComponent.SetPhysicsAsset` (`self.SK_Door`) "/Game/AdvancedLocomotionV4/Props/Environment_Props/Wardrobe/SK_Wardrobe_PhysicsAsset.SK_Wardrobe_PhysicsAsset" true)
      (`BoxComponent.SetBoxExtent` (`self.Trigger`) (40.0 30.0 60.0) true)
      (`SceneComponent.K2_SetRelativeLocation` (`self.Trigger`) (0.0 -28.0 60.0) false false)
      (`StaticMeshComponent.SetStaticMesh` (`self.AdditiveMesh`) "/Game/AdvancedLocomotionV4/Props/Environment_Props/Wardrobe/SM_Wardrobe_Part01.SM_Wardrobe_Part01")
      (`StaticMeshComponent.SetStaticMesh` (`self.AdditiveMesh2`) "/Game/AdvancedLocomotionV4/Props/Environment_Props/Wardrobe/SM_Wardrobe_Part02.SM_Wardrobe_Part02")
      (`SceneComponent.K2_SetRelativeLocation` (`self.WidgetOrigin`) (0.0 -8.0 120.0) false false)
      (`SceneComponent.K2_SetRelativeLocation` (`self.TargetCharLocation`) (0.0 -75.0 0.0) false false))))

(fn `Widget-Destroy`
  (`self.InfoWidgetObject`
    (:`then`
      (`Widget.SetVisibility` (`self.InfoWidgetObject`) "Hidden")
      (`Widget.RemoveFromParent` (`self.InfoWidgetObject`))
      (set `self.GeneratedInfoWidget` false)
      (set `self.InfoWidgetObject` null)
      (`KismetSystemLibrary.K2_ClearTimer` null "CheckWhdgetWhenInTrigger"))
    (:`else`)))

(fn `Widget-Generate`
  (params (Actor :type "Actor Object Reference"))
  (returns (generate :type Boolean))
  (locals (Character :type "Character Object Reference") (`Pistol Equal` :type Boolean))
  (bind _infowidgetobject (`self.InfoWidgetObject`))
  (bind _infowidgetobject_2 (`self.InfoWidgetObject`))
  (bind _ascharacter (cast `Character` Actor))
  (set `local.Character` _ascharacter)
  (if (`Pawn.IsPlayerControlled` _ascharacter)
    (bind _returnvalue (message `/Game/AdvancedLocomotionV4/Blueprints/Interfaces/ALS_PlayerCharacter_BPI.PBPI_CheckItemCanSpawnWidget` (`local.Character`) self (`self.K2_GetActorLocation`)))
    (if _returnvalue
      (if (and (`self.IsClosed`) (not (`self.GeneratedInfoWidget`)))
        ;[1 1 1] Spawn Widget
        (bind _returnvalue_2 (`|CreateWidget` "/Game/AdvancedLocomotionV4/Blueprints/UI/Item_Information_UI.Item_Information_UI_C"))
        (bind _output_get (set `self.InfoWidgetObject` _returnvalue_2))
        (`UserWidget.AddToViewport` _output_get -1)
        (set `self.GeneratedInfoWidget` true)
        (`UserWidget.PlayAnimation` _infowidgetobject (`/Game/AdvancedLocomotionV4/Blueprints/UI/Item_Information_UI.Fade_In` _infowidgetobject) 0.0 1 "Forward" 1.4 false)
        (`|ExecutionSequence`
          (:`then_0`
            ;[1 1 1] Updare String
            (`TextBlock.SetText` (`/Game/AdvancedLocomotionV4/Blueprints/UI/Item_Information_UI.T_Title` (`self.InfoWidgetObject`)) "")
            (`TextBlock.SetText` (`/Game/AdvancedLocomotionV4/Blueprints/UI/Item_Information_UI.T_Comment` (`self.InfoWidgetObject`)) "")
            (`Widget.SetRenderOpacity` (`/Game/AdvancedLocomotionV4/Blueprints/UI/Item_Information_UI.BG_Blur` (`self.InfoWidgetObject`)) 0.0))
          (:`then_1`
            ;[1 1 1] Play Animation
            (`UserWidget.PlayAnimation` _infowidgetobject_2 (`/Game/AdvancedLocomotionV4/Blueprints/UI/Item_Information_UI.Button_Loop` _infowidgetobject_2) 0.0 15 "Forward" 1.4 false)
            (`KismetSystemLibrary.K2_SetTimer` null "Widget Update Event" 0.01 true))
          (:`then_2`
            ;[1 1 1] Activate Tick
            (`ActorComponent.SetComponentTickInterval` (`self.SK_Door`) 0.0)))
        (else
          (return false)))
      (else
        (`KismetSystemLibrary.K2_SetTimer` null "CheckWhdgetWhenInTrigger" 0.5)
        (return false)))
    (else
      (return false))))

(fn `Widget-Update`
  (if (and (`self.GeneratedInfoWidget`) (`KismetSystemLibrary.IsValid` (`self.InfoWidgetObject`)))
    (`KismetSystemLibrary.K2_ClearTimer` null "CheckWhdgetWhenInTrigger")
    (`CanvasPanelSlot.SetPosition` (`WidgetLayoutLibrary.SlotAsCanvasSlot` (`/Game/AdvancedLocomotionV4/Blueprints/UI/Item_Information_UI.MovablePanel` (`self.InfoWidgetObject`))) (`WidgetLayoutLibrary.ProjectWorldLocationToWidgetPosition` (`Widget.GetOwningPlayer` (`self.InfoWidgetObject`)) (+ (`SceneComponent.K2_GetComponentLocation` (`self.WidgetOrigin`)) (0.0 0.0 0.0))))
    (else
      (`KismetSystemLibrary.K2_ClearTimer` null "Widget Update Event"))))