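; Animation Modifier that adjusts the left and right upperarm_twist_01 bones in an animation sequence through transform curves.
; On apply, RefreshCurve removes any existing transform curve with each bone's name and adds an empty one, so reapplying starts clean.
; Each curve then gets a single key holding the inverse of that bone's sampled pose, with frame and time left at their defaults.
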(event `self.OnApply`
  (params (AnimationSequence :type "AnimSequence Object Reference"))
  (set `self.AnimSeq` AnimationSequence)
  (`self.RefreshCurve` "upperarm_twist_01_l")
  (`self.RefreshCurve` "upperarm_twist_01_r")
  (`AnimationBlueprintLibrary.AddTransformationCurveKey` (`self.AnimSeq`) "upperarm_twist_01_l" 0.0 (`KismetMathLibrary.InvertTransform` (`AnimationBlueprintLibrary.GetBonePoseForFrame` (`self.AnimSeq`) "upperarm_twist_01_l")))
  (`AnimationBlueprintLibrary.AddTransformationCurveKey` (`self.AnimSeq`) "upperarm_twist_01_r" 0.0 (`KismetMathLibrary.InvertTransform` (`AnimationBlueprintLibrary.GetBonePoseForFrame` (`self.AnimSeq`) "upperarm_twist_01_r"))))

(fn `RefreshCurve`
  (params (Name :type Name))
  (bind _animseq (`self.AnimSeq`))
  (bind _returnvalue (`AnimationBlueprintLibrary.DoesCurveExist` _animseq Name "RCT_Transform"))
  (if _returnvalue
    (`AnimationBlueprintLibrary.RemoveCurve` (`self.AnimSeq`) Name))
  (`AnimationBlueprintLibrary.AddCurve` _animseq Name "RCT_Transform"))